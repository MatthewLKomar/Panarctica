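; Actor that drifts through the world in successive random straight-line moves.
; MotionEnded picks a random offset from the current location and drives a Lerp timeline to move there without sweep.
; The timeline's play rate is a random speed divided by the offset length.
; Finishing re-triggers MotionEnded, so drift chains without a fixed anchor, though BeginPlay is empty and does not start it.
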(event Custom|Event%20MotionEnded
  (Variables|Default|SetLastLocation (Transformation|GetActorLocation))
  (bind (_destination _distance) (CallFunction|SetRandomDestination))
  (Components|Timeline|SetPlayRate (Variables|Default|GetLerp) (Math|Float|SafeDivide (Math|Random|RandomFloatinRange (Variables|Default|GetMinSpeed) (Variables|Default|GetMaxSpeed)) _distance))
  (bind _alpha (Timeline|Lerp PlayFromStart)
    (:Update
      (Transformation|SetActorLocation (Math|Vector|Lerp(Vector) (Variables|Default|GetLastLocation) _destination _alpha) false false))
    (:Finished
      (CallFunction|EventMotionEnded))))

(event EventBeginPlay)

(event Collision|EventActorBeginOverlap
  (params (OtherActor :type Actor%20Object%20Reference)))

(event EventTick
  (params (DeltaSeconds :type Float%20%28single-precision%29)))

(fn ConstructionScript)

(fn SetRandomDestination
  (bind _rangex (Variables|Default|GetRangeX))
  (bind _rangey (Variables|Default|GetRangeY))
  (bind _rangez (Variables|Default|GetRangeZ))
  (bind _rand (Utilities|RandFloatinRange _rangex))
  (bind _rand_2 (Utilities|RandFloatinRange _rangey))
  (bind _rand_3 (Utilities|RandFloatinRange _rangez))
  (bind _returnvalue (Math|Vector|MakeVector _rand _rand_2 _rand_3))
  (return (+ (Transformation|GetActorLocation) _returnvalue) (Math|Vector|VectorLength _returnvalue)))