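; Elevator actor that carries the player up once, with sliding double doors that open on BeginPlay.
; The first overlap of the platform trigger sets EnteredLift and reverses the door timelines to close them.
; The right door timeline's Finished pin then starts the Move timeline, which lerps the platform's relative location to PlatformEnd's height and calls OpenDoors on arrival.
; A DoOnce limits the trigger to one trip, with no return.
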(event OnComponentBeginOverlap(PlatformTrigger)
  (params (OverlappedComponent :type Primitive%20Component%20Object%20Reference) (OtherActor :type Actor%20Object%20Reference) (OtherComp :type Primitive%20Component%20Object%20Reference) (OtherBodyIndex :type Integer) (bFromSweep :type Boolean) (SweepResult :type Hit%20Result%20Structure%20%28by%20ref%29))
  ;[1 1 1] Someone's on the elevatore so move up
  (Utilities|FlowControl|DoOnce false
    (:Completed
      (Variables|Default|SetenteredLift true)
      (CallFunction|CloseDoors))))

(event Custom|OpenDoors
  (bind _left_door_enter_start (Variables|Default|GetLeft%20Door%20Enter%20Start))
  (bind _right_door_enter_start (Variables|Default|GetRight%20Door%20Enter%20Start))
  ;[1 1 1] Close the doors
  (Utilities|FlowControl|Sequence
    (:then_0
      (bind _newtrack_0 (Timeline|Left%20Door%20Enter Play)
        (:Update
          (Transformation|SetRelativeLocation (Variables|Default|GetLeft%20Door) (Math|Vector|Lerp(Vector) _left_door_enter_start (+ _left_door_enter_start (Math|Vector|MakeVector (Variables|Default|GetDoorOffset) 0.0 0.0)) _newtrack_0) false false))))
    (:then_1
      ;[1 1 1] Open the doors
      (bind _newtrack_0_2 (Timeline|Right%20Door%20Enter Play)
        (:Update
          (Transformation|SetRelativeLocation (Variables|Default|GetRight%20Door) (Math|Vector|Lerp(Vector) _right_door_enter_start (- _right_door_enter_start (Math|Vector|MakeVector (Variables|Default|GetDoorOffset) 0.0 0.0)) _newtrack_0_2) false false))
        (:Finished
          (if (Variables|Default|GetenteredLift)
            (CallFunction|MoveElevator)))))))

(event Custom|CloseDoors
  (bind _left_door_enter_start (Variables|Default|GetLeft%20Door%20Enter%20Start))
  (bind _right_door_enter_start (Variables|Default|GetRight%20Door%20Enter%20Start))
  ;[1 1 1] Open the doors
  (Utilities|FlowControl|Sequence
    (:then_0
      ;[1 1 1] Close the doors
      (bind _newtrack_0 (Timeline|Left%20Door%20Enter Reverse)
        (:Update
          (Transformation|SetRelativeLocation (Variables|Default|GetLeft%20Door) (Math|Vector|Lerp(Vector) _left_door_enter_start (+ _left_door_enter_start (Math|Vector|MakeVector (Variables|Default|GetDoorOffset) 0.0 0.0)) _newtrack_0) false false))))
    (:then_1
      (bind _newtrack_0_2 (Timeline|Right%20Door%20Enter Reverse)
        (:Update
          (Transformation|SetRelativeLocation (Variables|Default|GetRight%20Door) (Math|Vector|Lerp(Vector) _right_door_enter_start (- _right_door_enter_start (Math|Vector|MakeVector (Variables|Default|GetDoorOffset) 0.0 0.0)) _newtrack_0_2) false false))
        (:Finished
          (if (Variables|Default|GetenteredLift)
            (CallFunction|MoveElevator)))))))

(event Custom|MoveElevator
  ;[1 1 1] Someone's on the elevatore so move up
  (bind _newtrack_1 (Timeline|Move Play)
    (:Update
      (Transformation|SetRelativeLocation (Variables|Default|GetPlatform) (Math|Vector|Lerp(Vector) (Variables|Default|GetPlatform%20Start) (Variables|Default|GetPlatform%20End) _newtrack_1) false false))
    (:Finished
      (CallFunction|OpenDoors))))

(event EventBeginPlay
  (Variables|Default|SetLeft%20Door%20Enter%20Start (Variables|/Script/Engine.SceneComponent|GetRelativeLocation (Variables|Default|GetLeft%20Door)))
  (Variables|Default|SetRight%20Door%20Enter%20Start (Variables|/Script/Engine.SceneComponent|GetRelativeLocation (Variables|Default|GetRight%20Door)))
  (Variables|Default|SetElevatorStartPosition (Variables|/Script/Engine.SceneComponent|GetRelativeLocation (Variables|Default|GetPlatform)))
  (Variables|Default|SetPlatform%20Start (Variables|/Script/Engine.SceneComponent|GetRelativeLocation (Variables|Default|GetPlatform)))
  (Variables|Default|SetPlatform%20End (Math|Vector|MakeVector 0.0 0.0 (.z (Variables|Default|GetPlatform%20End))))
  (CallFunction|OpenDoors))

(fn ConstructionScript)