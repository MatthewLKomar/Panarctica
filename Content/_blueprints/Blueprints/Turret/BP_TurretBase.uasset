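; Base turret pawn that the first-person character can possess and aim.
; Overlapping InteractionZone binds the character's interact event to TryEnterTurret, which possesses the turret and hides the character; Dequip reverses this.
; Despite its name, FireGun starts a looping timer that rotates GunRoot toward the camera's look point.
; ZoomIn and ZoomOut are empty, and FireProjectile, which spawns a projectile with sound, is never called here.
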(event OnComponentBeginOverlap(InteractionZone)
  (params (OverlappedComponent :type Primitive%20Component%20Object%20Reference) (OtherActor :type Actor%20Object%20Reference) (OtherComp :type Primitive%20Component%20Object%20Reference) (OtherBodyIndex :type Integer) (bFromSweep :type Boolean) (SweepResult :type Hit%20Result%20Structure%20%28by%20ref%29))
  (bind _asbp_first_person_character (Utilities|Casting|CastToBP_FirstPersonCharacter OtherActor))
  (Development|PrintString "Press Q to interact" true true "(R=0.000000,G=0.660000,B=1.000000,A=1.000000)" 5.0)
  (EventDispatchers|BindEventtoOnInteract _asbp_first_person_character (delegate Custom|EquipAttempt)))

(event OnComponentEndOverlap(InteractionZone)
  (params (OverlappedComponent :type Primitive%20Component%20Object%20Reference) (OtherActor :type Actor%20Object%20Reference) (OtherComp :type Primitive%20Component%20Object%20Reference) (OtherBodyIndex :type Integer))
  (Development|PrintString "No More Interacting")
  (bind _asbp_first_person_character (Utilities|Casting|CastToBP_FirstPersonCharacter (Variables|Default|GetOriginalCharacter)))
  (EventDispatchers|UnbindEventfromOnInteract _asbp_first_person_character (delegate Custom|EquipAttempt)))

(event Custom|FireGun
  (bind _returnvalue (Utilities|Time|SetTimerbyFunctionName 0 "CheckWhereToShoot" 0.01 true))
  (Variables|Default|SetFiringGun _returnvalue))

(event Custom|EquipAttempt
  (params (SelfReference :type BP%20First%20Person%20Character%20Object%20Reference))
  (Development|PrintString "try equip")
  (CallFunction|TryEnterTurret SelfReference))

(event EventBeginPlay)

(event Input|ActionEvents|InputActionSecondaryAction
  (params (Key :type Key%20Structure :default "None"))
  (:Pressed
    (CallFunction|Zoomin))
  (:Released
    (CallFunction|ZoomOut)))

(event Input|ActionEvents|InputActioneQuip
  (params (Key :type Key%20Structure :default "None"))
  (:Pressed
    (CallFunction|Dequip)))

(fn ConstructionScript)

(fn Zoomin)

(fn ZoomOut)

(fn FireProjectile
  (params (OriginPoint :type Vector))
  ;[0.05 0.05 0.05] Projectile Spawn Logic
  (Game|SpawnActorfromClass "/Game/_blueprints/Blueprints/BP_FirstPersonProjectile.BP_FirstPersonProjectile_C" (Math|Transform|MakeTransform OriginPoint (Camera|GetCameraRotation (Game|GetPlayerCameraManager 0))) "Undefined" 0 0)
  (Audio|PlaySoundatLocation "/Game/_assets/FPWeapon/Audio/FirstPersonTemplateWeaponFire02.FirstPersonTemplateWeaponFire02" OriginPoint "0, 0, 0" 1.0 1.0 0.0 0 0 0 0) ; Play firing sound
)

(fn CheckWheretoShoot
  (bind _returnvalue (Game|GetPlayerCameraManager 0))
  (Variables|Default|SetLookLocation (+ (* (Math|Vector|GetForwardVector (Transformation|GetActorRotation _returnvalue)) (Class|KismetSystemLibrary|MakeLiteralInteger 1000)) (Transformation|GetActorLocation _returnvalue)))
  (Transformation|SetRelativeRotation (Variables|Default|GetGunRoot) (Math|Rotator|MakeRotator 0.0 (.Pitch (Math|Rotator|BreakRotator (Math|Rotator|MakeRotfromX (Math|Transform|InverseTransformDirection (Transformation|GetActorTransform) (- (Variables|Default|GetLookLocation) (Transformation|GetWorldLocation (Variables|Default|GetGunRoot))))))) (.Yaw (Math|Rotator|BreakRotator (Math|Rotator|MakeRotfromX (Math|Transform|InverseTransformDirection (Transformation|GetActorTransform) (- (Variables|Default|GetLookLocation) (Transformation|GetWorldLocation (Variables|Default|GetGunRoot)))))))) false false))

(fn Equip
  (params (OwningCharacter :type Pawn%20Object%20Reference))
  (Variables|Default|SetOriginalCharacter OwningCharacter)
  (CallFunction|FireGun))

(fn Dequip
  (bind _returnvalue (Game|GetPlayerController 0))
  (bind _firinggun (Variables|Default|GetFiringGun))
  (bind _originalcharacter (Variables|Default|GetOriginalCharacter))
  (Utilities|FlowControl|Sequence
    (:then_0
      ;[1 1 1] Stop Looking Where To Shoot
      (if (Utilities|Time|IsValidTimerHandle _firinggun)
        (Utilities|Time|ClearandInvalidateTimerbyHandle _firinggun)
        (else
          (Development|PrintString "invalid"))))
    (:then_1
      (Collision|SetActorEnableCollision _originalcharacter true)
      (Actor|Tick|SetActorTickEnabled _originalcharacter true)
      (Rendering|SetActorHiddenInGame _originalcharacter false)
      ;[1 1 1] Un-Possess ourselves and reposses the player
      (Pawn|UnPossess _returnvalue)
      (Pawn|Possess _returnvalue (Variables|Default|GetOriginalCharacter)))))

(fn TryEnterTurret
  (params (OwningCharacter :type Pawn%20Object%20Reference))
  (bind _originalcharacter (Variables|Default|GetOriginalCharacter))
  (LocalVariables|SetCurrentPlayerController (Pawn|GetController OwningCharacter))
  (Pawn|UnPossess (LocalVariables|GetCurrentPlayerController))
  (Pawn|Possess (LocalVariables|GetCurrentPlayerController) self)
  (CallFunction|Equip OwningCharacter)
  (Collision|SetActorEnableCollision _originalcharacter false)
  (Actor|Tick|SetActorTickEnabled _originalcharacter)
  (Components|Movement|StopMovementImmediately (Pawn|GetMovementComponent _originalcharacter))
  (Rendering|SetActorHiddenInGame _originalcharacter true))