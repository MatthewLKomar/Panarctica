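; Hook projectile fired by BP_GrappleTurret, with a cable attached on spawn to the turret's gun.
; A sphere collision hit on a BP_ValidVolume stops the projectile, records the grapple point, moves the cable end to the turret's grapple surface attach point and notifies the turret.
; Any other hit destroys the hook and reports a miss, with a timer apparently doing the same when nothing is hit.
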(event OnComponentHit(SphereCollision)
  (params (HitComponent :type Primitive%20Component%20Object%20Reference) (OtherActor :type Actor%20Object%20Reference) (OtherComp :type Primitive%20Component%20Object%20Reference) (NormalImpulse :type Vector :default "0, 0, 0") (Hit :type Hit%20Result%20Structure%20%28by%20ref%29))
  (Rendering|Debug|DrawDebugSphere (Transformation|GetActorLocation OtherActor) 1e+02 12 "(R=1.000000,G=0.000000,B=0.000000,A=1.000000)" 3e+01)
  (Utilities|Casting|CastToBP_ValidVolume OtherActor
    (:then
      (CallFunction|OnHitTarget)
      (Default|TargetHit (Variables|Default|GetTurret))
      (Variables|Default|SetisHit true))
    (:CastFailed
      (CallFunction|TargetMissed)
      (Variables|Default|SetisHit false))))

(event Custom|OnHitTarget
  (bind _projectilemovement (Variables|Default|GetProjectileMovement))
  (Components|Movement|StopMovementImmediately _projectilemovement)
  (Variables|/Script/Engine.ProjectileMovementComponent|SetProjectileGravityScale _projectilemovement 0.0)
  (Variables|Default|SetGrapplePoint (Transformation|GetActorLocation))
  (Variables|Default|SetIsGrappled true)
  (bind _asbp_attach_grapple (Utilities|Casting|CastToBP_AttachGrapple (Variables|/Game/_blueprints/Blueprints/Turret/BP_GrappleTurret.BP_GrappleTurret_C|GetGrappleSurface (Variables|Default|GetTurret))))
  (Class|CableComponent|SetAttachEndtoComponent (Variables|Default|GetCable) (Variables|/Game/_blueprints/Blueprints/Turret/BP_AttachGrapple.BP_AttachGrapple_C|GetAttachPoint _asbp_attach_grapple) "joint1"))

(event Custom|DestroyIfNotHit
  (if (not (Variables|Default|GetisHit))
    (CallFunction|TargetMissed)))

(event EventBeginPlay
  (bind _asbp_grapple_turret (Utilities|Casting|CastToBP_GrappleTurret (Game|GetInstigator)))
  (Variables|Default|SetTurret _asbp_grapple_turret)
  (Class|CableComponent|SetAttachEndtoComponent (Variables|Default|GetCable) (Variables|/Game/_blueprints/Blueprints/Turret/Templates/BP_TurretBase.BP_TurretBase_C|GetGun _asbp_grapple_turret) "joint1")
  (Utilities|Time|SetTimerbyEvent (EventDispatchers|CreateEvent :!event Custom|DestroyIfNotHit) 0.1 false 3.0))

(fn ConstructionScript)

(fn TargetMissed
  (Actor|DestroyActor)
  (Default|TargetMissed (Variables|Default|GetTurret)))