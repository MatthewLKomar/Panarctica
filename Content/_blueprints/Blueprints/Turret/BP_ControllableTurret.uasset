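; Player-controllable turret whose gun follows where the player's camera looks.
; Mouse axes rotate the Camera in yaw and pitch within fixed limits via IsWithinBounds, while a keyboard axis adds clamped controller yaw.
; Tick projects a point ahead of the player camera and rotates GunRoot toward it in actor-local space, without roll.
; SecondaryAction press and release set a flag that is not read here.
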(event EventTick
  (params (DeltaSeconds :type Float%20%28single-precision%29))
  (bind _returnvalue (Game|GetPlayerCameraManager 0))
  (Variables|Default|SetLookLocation (+ (* (Math|Vector|GetForwardVector (Transformation|GetActorRotation _returnvalue)) (Class|KismetSystemLibrary|MakeLiteralInteger 1000)) (Transformation|GetActorLocation _returnvalue)))
  (Transformation|SetRelativeRotation (Variables|Default|GetGunRoot) (Math|Rotator|MakeRotator 0.0 (.Pitch (Math|Rotator|BreakRotator (Math|Rotator|MakeRotfromX (Math|Transform|InverseTransformDirection (Transformation|GetActorTransform) (- (Variables|Default|GetLookLocation) (Transformation|GetWorldLocation (Variables|Default|GetGunRoot))))))) (.Yaw (Math|Rotator|BreakRotator (Math|Rotator|MakeRotfromX (Math|Transform|InverseTransformDirection (Transformation|GetActorTransform) (- (Variables|Default|GetLookLocation) (Transformation|GetWorldLocation (Variables|Default|GetGunRoot)))))))) false false))

(event Input|ActionEvents|InputActionSecondaryAction
  (params (Key :type Key%20Structure :default "None"))
  ;[1 1 1] Free look to control the gun
  (:Pressed
    (Variables|Default|SetSecondaryAction true))
  (:Released
    (Variables|Default|SetSecondaryAction false)))

(event Input|AxisEvents|InputAxisMoveRight/Left
  (params (AxisValue :type Float%20%28single-precision%29))
  ;[1 1 1] Keyboard Input alternative:
  (Pawn|Input|AddControllerYawInput (Math|Float|Clamp(Float) AxisValue -0.5 0.5)))

(event Input|AxisEvents|InputAxisTurnRight/LeftMouse
  (params (AxisValue :type Float%20%28single-precision%29))
  (bind _camera (Variables|Default|GetCamera))
  (bind _relativerotation (Variables|/Script/Engine.SceneComponent|GetRelativeRotation _camera))
  (bind _returnvalue (+ AxisValue (.yaw _relativerotation)))
  ;[0.05 0.05 0.05] Movement of the Gun: Yaw and Pitch Input - Mouse
  (Utilities|IsWithinBounds -35.0 35.0 _returnvalue
    (:true
      (Transformation|SetRelativeRotation (Variables|Default|GetCamera) (Math|Rotator|MakeRotator (.roll _relativerotation) (.pitch _relativerotation) _returnvalue) false false))))

(event Input|AxisEvents|InputAxisLookUp/DownMouse
  (params (AxisValue :type Float%20%28single-precision%29))
  (bind _returnvalue (* AxisValue -1.0))
  (bind _camera (Variables|Default|GetCamera))
  (bind _relativerotation (Variables|/Script/Engine.SceneComponent|GetRelativeRotation _camera))
  (bind _returnvalue_2 (+ _returnvalue (.pitch _relativerotation)))
  ;[0.05 0.05 0.05] Movement of the Gun: Yaw and Pitch Input - Mouse
  (Utilities|IsWithinBounds -35.0 35.0 _returnvalue_2
    (:true
      (Transformation|SetRelativeRotation (Variables|Default|GetCamera) (Math|Rotator|MakeRotator (.roll _relativerotation) _returnvalue_2 (.yaw _relativerotation)) false false))))

(fn ConstructionScript)