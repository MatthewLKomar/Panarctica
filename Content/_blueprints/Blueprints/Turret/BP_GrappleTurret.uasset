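; Player-operated grapple turret that fires a BP_HookProjectile to set up a zipline ride.
; Yaw input turns the controller and mouse up/down rotates the gun; firing locks until the reload montage completes, toggling zoom around it.
; A Zoom timeline lerps the camera between hip and sight views, reparenting it between CameraRoot and Gun.
; TargetHit starts ZiplineManager and dequips the turret, while TargetMissed plays a hint sound.
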(event Custom|FireGun
  ;[1 1 1] Fire Control
  ;;[1 1 1] Fire the Gun
  (if (not (Variables|Default|GetIsReloading))
    (bind _returnvalue (CallFunction|FireProjectile (Transformation|GetWorldLocation (Variables|Default|GetMuzzle))))
    (CallFunction|ConfigureProjectile _returnvalue)
    (Variables|Default|SetIsReloading true)
    ;;[1 1 1] Play the cool animations
    (Components|Animation|PlayAnimation (Variables|Default|GetGun) "/Game/_assets/Guns/GrappleCannon/Canon_Reloading.Canon_Reloading" false)
    (Animation|Montage|PlayMontage (Variables|Default|GetHands) "/Game/_assets/FPHands/Animations/Cannon/Reload_CanonHands_Montage.Reload_CanonHands_Montage"
      (:then
        ;;[1 1 1] Zoom in/out during reload sequence
        (CallFunction|HandleZoom)
        (Variables|Default|SetIsReloading true))
      (:OnCompleted
        (Variables|Default|SetIsReloading false)
        (CallFunction|HandleZoom)))))

(event Custom|HandleZoom
  ;[1 1 1] Fire Control
  ;;[1 1 1] Zoom Functionality
  (Variables|Default|SetIsZoomingIn true)
  (CallFunction|SetupCameraforAimDown)
  (bind _newtrack_0 (Timeline|Zoom PlayFromStart)
    (:Update
      (CallFunction|AimDownSightLogic _newtrack_0))
    (:Finished
      (Variables|Default|SetIsZoomingIn false)
      (if (Variables|Default|GetZoomedIn)
        (Variables|Default|SetZoomedIn false)
        (else
          (Variables|Default|SetZoomedIn true))))))

(event EventOnDequiped
  ;[1 1 1] Equip/Dequp Logic
  (Development|SetHiddeninGame (Variables|Default|GetHands) false true))

(event EventOnEquiped
  ;[1 1 1] Equip/Dequp Logic
  (Development|SetHiddeninGame (Variables|Default|GetHands) false true)
  (CallFunction|HandleZoom))

(event EventBeginPlay
  (Variables|Default|SetProjectile "/Game/_blueprints/Blueprints/Turret/BP_HookProjectile.BP_HookProjectile_C"))

(event Input|ActionEvents|InputActionSecondaryAction
  (params (Key :type Key%20Structure :default "None"))
  ;[1 1 1] Fire Control
  ;;[1 1 1] RMB to zoom toggle
  (:Pressed
    (if (not (Variables|Default|GetIsZoomingIn))
      (CallFunction|HandleZoom))))

(event Input|AxisEvents|InputAxisMoveRight/Left
  (params (AxisValue :type Float%20%28single-precision%29))
  ;[1 1 1] Move the Yaw of the turret
  (Pawn|Input|AddControllerYawInput (Math|Float|Clamp(Float) AxisValue -0.1 0.1)))

(event Input|AxisEvents|InputAxisLookUp/DownMouse
  (params (AxisValue :type Float%20%28single-precision%29))
  ;[0.05 0.05 0.05] Camera Yaw and Pitch rotation movement
  (CallFunction|CalculateGunRot AxisValue))

(event Input|MouseEvents|LeftMouseButton
  (params (Key :type Key%20Structure :default "None"))
  ;[1 1 1] Fire Control
  (:Pressed
    (CallFunction|FireGun)))

(fn ConstructionScript)

(fn CalculateCamera
  (params (DeltaInput :type Float%20%28double-precision%29))
  (bind _returnvalue (* DeltaInput -1.0))
  (bind _camera (Variables|Default|GetCamera))
  (bind _relativerotation (Variables|/Script/Engine.SceneComponent|GetRelativeRotation _camera))
  (bind _returnvalue_2 (+ _returnvalue (.pitch _relativerotation)))
  (Utilities|IsWithinBounds (Variables|Default|GetMinPitchVal) (Variables|Default|GetMaxPitchVal) _returnvalue_2
    (:true
      (Transformation|SetRelativeRotation (Variables|Default|GetCamera) (Math|Rotator|MakeRotator (.roll _relativerotation) _returnvalue_2 (.yaw _relativerotation)) false false))))

(fn CalculateGunRot
  (params (A :type Float%20%28double-precision%29))
  (bind _gun (Variables|Default|GetGun))
  (bind _relativerotation (Variables|/Script/Engine.SceneComponent|GetRelativeRotation _gun))
  (Utilities|IsWithinBounds (Variables|Default|GetMinPitchVal) (Variables|Default|GetMaxPitchVal) A
    (:true
      (Transformation|SetRelativeRotation (Variables|Default|GetGun) (Math|Rotator|MakeRotator (+ A (.roll _relativerotation)) (.pitch _relativerotation) (.yaw _relativerotation)) false false))))

(fn AimDownSightLogic
  (params (Alpha :type Float%20%28single-precision%29))
  (if (not (Variables|Default|GetZoomedIn))
    (Transformation|SetRelativeLocation (Variables|Default|GetCamera) (Math|Vector|Lerp(Vector) (Variables|/Script/Engine.SceneComponent|GetRelativeLocation (Variables|Default|GetCamera)) (Variables|/Script/Engine.SceneComponent|GetRelativeLocation (Variables|Default|GetAimDownSight)) Alpha) false false)
    (else
      (Transformation|SetRelativeLocation (Variables|Default|GetCamera) (Math|Vector|Lerp(Vector) (Variables|/Script/Engine.SceneComponent|GetRelativeLocation (Variables|Default|GetAimDownSight)) "0, 0, 0" Alpha) false false))))

(fn SetupCameraforAimDown
  (bind _camera (Variables|Default|GetCamera))
  (if (Variables|Default|GetZoomedIn)
    (Transformation|AttachComponentToComponent (Variables|Default|GetCamera) (Variables|Default|GetCameraRoot) "None" "KeepWorld" "KeepRelative" "KeepRelative" false)
    (Transformation|SetRelativeRotation _camera "0.000000,0.000000,0.000000" false false)
    (else
      (Transformation|AttachComponentToComponent (Variables|Default|GetCamera) (Variables|Default|GetGun) "None" "KeepWorld" "SnapToTarget" "KeepRelative" true)
      (Transformation|SetRelativeRotation _camera "0.000000,90.000000,0.000000" false false))))

(fn ConfigureProjectile
  (params (Object :type Object%20Object%20Reference))
  (bind _asbp_hook_projectile (Utilities|Casting|CastToBP_HookProjectile Object))
  (Variables|Default|Setgrapple_hook _asbp_hook_projectile))

(fn TargetHit
  (params (target :type Vector))
  (Audio|PlaySound2D "/Game/_assets/audio/Prof/CannonSequence/Great_Job.Great_Job" 1.0 1.0 0.0 0 0)
  (Variables|Default|SetisEquippable false)
  (Development|SetHiddeninGame (Variables|Default|GetHands) true false)
  (Default|StartZiplining (Variables|Default|GetZiplineManager) target)
  (CallFunction|Dequip))

(fn TargetMissed
  (Audio|PlaySound2D "/Game/_assets/audio/Prof/CannonSequence/Aim_For_The_Smokestack.Aim_For_The_Smokestack" 1.0 1.0 0.0 0 0))