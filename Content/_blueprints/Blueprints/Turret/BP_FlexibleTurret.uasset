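; BP_FlexibleTurret is a player-controlled twin-barrel turret that aims with the mouse and fires projectiles.
; Holding left mouse runs a looping FireRate timer on FireGun, cleared on release; a FlipFlop alternates shots between the two projectile start points.
; Mouse axes drive controller yaw and pitch, each clamped by MaxSpeed to cap turn speed.
; An IsWithinBounds range-check helper is defined but not called in these graphs.
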(event Custom|FireGun
  ;[1 1 1] Fire Control
  ;;[1 1 1] Flip between left and right guns
  (Utilities|FlowControl|FlipFlop
    (:A
      (CallFunction|FireProjectile (Transformation|GetWorldLocation (Variables|Default|GetProjectileStartPoint1))))
    (:B
      (CallFunction|FireProjectile (Transformation|GetWorldLocation (Variables|Default|GetProjectileStartPoint2))))))

(event Input|AxisEvents|InputAxisTurnRight/LeftMouse
  (params (AxisValue :type Float%20%28single-precision%29))
  (bind _maxspeed (Variables|Default|GetMaxSpeed))
  ;[0.05 0.05 0.05] Movement of the Gun: Yaw and Pitch Input - Mouse
  (Pawn|Input|AddControllerYawInput (Math|Float|Clamp(Float) AxisValue (* _maxspeed -1.0) _maxspeed)))

(event Input|AxisEvents|InputAxisLookUp/DownMouse
  (params (AxisValue :type Float%20%28single-precision%29))
  (bind _maxspeed (Variables|Default|GetMaxSpeed))
  ;[0.05 0.05 0.05] Movement of the Gun: Yaw and Pitch Input - Mouse
  (Pawn|Input|AddControllerPitchInput (Math|Float|Clamp(Float) AxisValue (* _maxspeed -1.0) _maxspeed)))

(event Input|MouseEvents|LeftMouseButton
  (params (Key :type Key%20Structure))
  ;[1 1 1] Fire Control
  ;;[1 1 1] press and hold the mouse to fire the gun
  (:Pressed
    (bind _returnvalue (Utilities|Time|SetTimerbyEvent (delegate Custom|FireGun) (Variables|Default|GetFireRate) true))
    (Variables|Default|SetFireLoop _returnvalue))
  (:Released
    (Utilities|Time|ClearandInvalidateTimerbyHandle (Variables|Default|GetFireLoop))))

(fn ConstructionScript)