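; BP_HeavyTurret is a player-controlled turret that fires a projectile from ProjectileStartPoint when the primary action is pressed.
; Mouse axes rotate the camera's relative yaw and pitch, with pitch input inverted, applying changes only when IsWithinBounds finds them strictly inside the min/max limits.
; The Move Right / Left axis separately turns the turret through controller yaw input, clamped to limit each step.
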(event Input|ActionEvents|InputActionPrimaryAction
  (params (Key :type Key%20Structure :default "None"))
  (:Pressed
    (CallFunction|FireProjectile (Transformation|GetWorldLocation (Variables|Default|GetProjectileStartPoint)))))

(event Input|AxisEvents|InputAxisMoveRight/Left
  (params (AxisValue :type Float%20%28single-precision%29))
  ;[1 1 1] Move the Yaw of the turret
  (Pawn|Input|AddControllerYawInput (Math|Float|Clamp(Float) AxisValue -0.5 0.5)))

(event Input|AxisEvents|InputAxisLookUp/DownMouse
  (params (AxisValue :type Float%20%28single-precision%29))
  (bind _returnvalue (* AxisValue -1.0))
  (bind _camera (Variables|Default|GetCamera))
  (bind _relativerotation (Variables|/Script/Engine.SceneComponent|GetRelativeRotation _camera))
  (bind _returnvalue_2 (+ _returnvalue (.pitch _relativerotation)))
  ;[0.05 0.05 0.05] Camera Yaw and Pitch rotation movement
  (Utilities|IsWithinBounds (Variables|Default|GetMinPitchVal) (Variables|Default|GetMaxPitchVal) _returnvalue_2
    (:true
      (Transformation|SetRelativeRotation (Variables|Default|GetCamera) (Math|Rotator|MakeRotator (.roll _relativerotation) _returnvalue_2 (.yaw _relativerotation)) false false))))

(event Input|AxisEvents|InputAxisTurnRight/LeftMouse
  (params (AxisValue :type Float%20%28single-precision%29))
  (bind _camera (Variables|Default|GetCamera))
  (bind _relativerotation (Variables|/Script/Engine.SceneComponent|GetRelativeRotation _camera))
  (bind _returnvalue (+ AxisValue (.yaw _relativerotation)))
  ;[0.05 0.05 0.05] Camera Yaw and Pitch rotation movement
  (Utilities|IsWithinBounds (Variables|Default|GetMinYawVal) (Variables|Default|GetMaxYawVal) _returnvalue
    (:true
      (Transformation|SetRelativeRotation (Variables|Default|GetCamera) (Math|Rotator|MakeRotator (.roll _relativerotation) (.pitch _relativerotation) _returnvalue) false false))))

(fn ConstructionScript)