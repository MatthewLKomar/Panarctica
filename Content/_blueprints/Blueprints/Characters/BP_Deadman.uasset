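; BP_Deadman is a damageable character that ragdolls on death and prints joke debug messages.
; BeginPlay binds the health component's damage and death events, with damage printing the amount taken.
; Death disables capsule collision and simulates physics below the Hips bone, then turns off mesh ticking after ten seconds.
; A Box overlap only prints a proximity warning; an unconnected player-triggered ragdoll chain never runs.
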(event OnComponentBeginOverlap(Box)
  (params (OverlappedComponent :type Primitive%20Component%20Object%20Reference) (OtherActor :type Actor%20Object%20Reference) (OtherComp :type Primitive%20Component%20Object%20Reference) (OtherBodyIndex :type Integer) (bFromSweep :type Boolean) (SweepResult :type Hit%20Result%20Structure%20%28by%20ref%29))
  (Development|PrintString "woah, too close bro!"))

(event Custom|Hurt
  (params (Damage :type Float%20%28double-precision%29))
  (Development|PrintString (Class|KismetStringLibrary|BuildStringDouble "" "Ow: " Damage)))

(event Custom|Tragedy
  (bind _mesh (Variables|Character|GetMesh))
  (Collision|SetCollisionEnabled (Variables|Default|GetCapsuleComponent) "NoCollision")
  (Collision|SetCollisionEnabled _mesh "QueryAndPhysics")
  (Class|SkeletalMeshComponent|SetAllBodiesBelowSimulatePhysics _mesh (Utilities|Name|MakeLiteralName "Hips") true true)
  (Components|Tick|SetComponentTickEnabled _mesh true)
  (Utilities|FlowControl|Delay 1e+01)
  (Components|Tick|SetComponentTickEnabled (Variables|Character|GetMesh) false)
  (Development|PrintString "Death has taken me, oh the tragedy"))

(event EventBeginPlay
  (bind _bp_pawnhealthcomponent1 (Variables|Default|GetBP_PawnHealthComponent1))
  (|CallParentFunction)
  (EventDispatchers|BindEventtoOnDamage _bp_pawnhealthcomponent1 (delegate Custom|Hurt))
  (EventDispatchers|BindEventtoDeath _bp_pawnhealthcomponent1 (delegate Custom|Tragedy)))

(event Collision|EventActorBeginOverlap
  (params (OtherActor :type Actor%20Object%20Reference))
  (|CallParentFunction OtherActor) ; This node is disabled and will not be called.\nDrag off pins to build functionality.
)

(event EventTick
  (params (DeltaSeconds :type Float%20%28single-precision%29))
  (|CallParentFunction DeltaSeconds) ; This node is disabled and will not be called.\nDrag off pins to build functionality.
)

(fn ConstructionScript
  (|CallParentFunction))