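; BP_ShotgunGuy is an enemy character that fires projectiles at the player's head.
; Tick calls Shoot when IsShooting is set, then clears the flag for single fire; the cooldown check is only a placeholder.
; Shoot plays a montage and sound, spawns a BP_FirstPersonProjectile at the gun's muzzle carrying GunDamage, and calls EndShoot.
; Overlapping any projectile it did not instigate destroys both the projectile and itself.
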(event EventBeginPlay
  (|CallParentFunction) ; This node is disabled and will not be called.\nDrag off pins to build functionality.
)

(event Collision|EventActorBeginOverlap
  (params (OtherActor :type Actor%20Object%20Reference))
  (Utilities|Casting|CastToBP_FirstPersonProjectile OtherActor)
  (if (!= (Variables|/Script/Engine.Actor|GetInstigator OtherActor) self)
    (Actor|DestroyActor OtherActor)
    (Actor|DestroyActor)))

(event EventTick
  (params (DeltaSeconds :type Float%20%28single-precision%29))
  (|CallParentFunction DeltaSeconds)
  (if (and (Variables|Default|GetIsShooting) true)
    (CallFunction|Shoot)
    (Variables|Default|SetIsShooting false) ; Single fire, so automatically stop after firing once
  ))

(fn ConstructionScript
  (|CallParentFunction))

(fn Shoot
  (bind _gunmesh (Variables|Components|GetGunMesh))
  (bind _returnvalue (Transformation|GetSocketLocation _gunmesh "Muzzle"))
  (|CallParentFunction)
  (Animation|PlayAnimMontage "/Game/_assets/Characters/Enemies/ShotgunGuy/Animations/AM_ShotgunGuy_Shoot.AM_ShotgunGuy_Shoot" 1.0 "None")
  (bind _returnvalue_2 (Game|SpawnActorfromClass "/Game/_blueprints/Blueprints/BP_FirstPersonProjectile.BP_FirstPersonProjectile_C" (Math|Transform|MakeTransform _returnvalue (Math|Conversions|RotationFromXVector (Math|Vector|GetUnitDirection(Vector) _returnvalue (Transformation|GetSocketLocation (Variables|/Script/Engine.Character|GetMesh (Game|GetPlayerCharacter 0)) "head")))) "Undefined" 0 self))
  (Variables|/Game/_blueprints/Blueprints/BP_FirstPersonProjectile.BP_FirstPersonProjectile_C|SetDamage _returnvalue_2 (Variables|Default|GetGunDamage))
  (Audio|PlaySoundatLocation "/Game/_assets/Guns/DefaultGun/Audio/FirstPersonTemplateWeaponFire02.FirstPersonTemplateWeaponFire02" _returnvalue "0, 0, 0" 1.0 1.0 0.0 0 0 0 0)
  (CallFunction|EndShoot))