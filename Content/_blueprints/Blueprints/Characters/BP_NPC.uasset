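; BP_NPC is an NPC character that provides movement-speed and shooting-state functions.
; Three setters switch the CharacterMovement max walk speed between idle, angered and attack values.
; Shoot and EndShoot only toggle the IsShooting flag for animation, with EndShoot meant to follow each Shoot call.
; The event graph and construction script are empty, so nothing in this file calls these functions.
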(event EventBeginPlay)

(event Collision|EventActorBeginOverlap
  (params (OtherActor :type Actor%20Object%20Reference)))

(event EventTick
  (params (DeltaSeconds :type Float%20%28single-precision%29)))

(fn ConstructionScript)

(fn SetIdleMoveSpeed
  (Variables|/Script/Engine.CharacterMovementComponent|SetMaxWalkSpeed (Variables|Character|GetCharacterMovement) (Variables|Default|GetIdleMoveSpeed)))

(fn SetAngeredMoveSpeed
  (Variables|/Script/Engine.CharacterMovementComponent|SetMaxWalkSpeed (Variables|Character|GetCharacterMovement) (Variables|Default|GetAngeredMoveSpeed)))

(fn SetAttackMoveSpeed
  (Variables|/Script/Engine.CharacterMovementComponent|SetMaxWalkSpeed (Variables|Character|GetCharacterMovement) (Variables|Default|GetAttackMoveSpeed)))

(fn Shoot
  (Variables|Default|SetIsShooting true))

(fn EndShoot
  (Variables|Default|SetIsShooting false))