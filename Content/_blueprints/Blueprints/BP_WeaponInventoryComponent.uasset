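; Weapon inventory component that tracks per-weapon ammo status and switches the Primary slot between Rock, Paper and Gun.
; A Startup event seeds the inventory map with three acquired, loaded weapons and shows the current Primary weapon.
; Releasing C steps a looping MultiGate to rewrite the slot's row name.
; UpdateWeaponMesh looks that name up in the WeaponData table and swaps the Weapon's skeletal mesh.
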(event Custom|Startup
  (bind _weaponinventory (Variables|Default|GetWeaponInventory))
  (Utilities|FlowControl|Sequence
    (:then_0
      (Utilities|Map|Add _weaponinventory "NewEnumerator2" (Utilities|Struct|MakeS_WeaponStatus true 10 10)))
    (:then_1
      (Utilities|Map|Add _weaponinventory "NewEnumerator1" (Utilities|Struct|MakeS_WeaponStatus true 3 3)))
    (:then_2
      (Utilities|Map|Add _weaponinventory "NewEnumerator0" (Utilities|Struct|MakeS_WeaponStatus true 3 3)))
    (:then_3
      (Utilities|UpdateWeaponMesh (.Value (Utilities|Map|Find (Variables|Default|GetWeaponSlots) "Primary"))))))

(event Input|KeyboardEvents|C
  (params (Key :type Key%20Structure :default "None"))
  (bind _weaponslots (Variables|Default|GetWeaponSlots))
  (:Released
    (Utilities|FlowControl|Sequence
      (:then_0
        (Utilities|FlowControl|MultiGate false true 0
          (:Out%200
            (Utilities|Map|Add _weaponslots "Primary" "Rock"))
          (:Out%201
            (Utilities|Map|Add _weaponslots "Primary" "Paper"))
          (:Out%202
            (Utilities|Map|Add _weaponslots "Primary" "Gun"))))
      (:then_1
        (Utilities|UpdateWeaponMesh (.Value (Utilities|Map|Find (Variables|Default|GetWeaponSlots) "Primary")))))))