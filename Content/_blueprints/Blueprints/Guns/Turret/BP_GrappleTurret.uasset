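; Mountable grapple turret that fires a hook projectile to start the player on a zipline.
; Mouse and axis input aim gun pitch and turret yaw within limits, while a timeline-driven toggle moves the camera for aim-down-sights.
; Firing locks aiming and zooms out during the reload montage.
; A hit disables re-equipping, hands off to ZiplineManager and dequips; a miss plays a hint voice line.
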(event Custom|FireGun
  ;[1 1 1] Fire Control
  ;;[1 1 1] Fire the Gun
  (if (not (Variables|Default|GetIsReloading))
    (bind _returnvalue (CallFunction|FireProjectile (Transformation|GetWorldLocation (Variables|Components|GetMuzzle))))
    (CallFunction|ConfigureProjectile _returnvalue)
    (Variables|Default|SetIsReloading true)
    ;;[1 1 1] Play the cool animations
    (Components|Animation|PlayAnimation (Variables|Default|GetGun) "/Game/_assets/Guns/GrappleCannon/Canon_Reloading.Canon_Reloading" false)
    (Animation|Montage|PlayMontage (Variables|Components|GetHands) "/Game/_assets/FPHands/Animations/Cannon/Reload_CanonHands_Montage.Reload_CanonHands_Montage"
      (:then
        ;;[1 1 1] Zoom in/out during reload sequence
        (if (Variables|Default|GetZoomedIn)
          (CallFunction|HandleZoom)
          (Variables|Default|SetIsReloading true)))
      (:OnCompleted
        (Variables|Default|SetIsReloading false)))))

(event Custom|HandleZoom
  ;[1 1 1] Fire Control
  ;;[1 1 1] Zoom Functionality
  (Variables|Default|SetIsZoomingIn true)
  (CallFunction|SetupCameraforAimDown)
  (bind _newtrack_0 (Timeline|Zoom PlayFromStart)
    (:Update
      (CallFunction|AimDownSightLogic _newtrack_0))
    (:Finished
      (Variables|Default|SetIsZoomingIn false)
      (if (Variables|Default|GetZoomedIn)
        (Variables|Default|SetZoomedIn false)
        (else
          (Variables|Default|SetZoomedIn true))))))

(event Custom|On%20Component%20Begin%20Overlap
  (params (OverlappedComponent :type Primitive%20Component%20Object%20Reference) (OtherActor :type Actor%20Object%20Reference) (OtherComp :type Primitive%20Component%20Object%20Reference) (OtherBodyIndex :type Integer) (bFromSweep :type Boolean) (SweepResult :type Hit%20Result%20Structure%20%28by%20ref%29))
  ;[1 1 1] Check for holding weapon before allowing task to update
  (bind _asbp_first_person_character (Utilities|Casting|CastToBP_FirstPersonCharacter OtherActor))
  (if (Variables|/Game/_blueprints/Blueprints/PlayableCharacters/BP_FirstPersonCharacter.BP_FirstPersonCharacter_C|GetIsWeaponDrawn _asbp_first_person_character)
    (Default|OnComponentBeginOverlapEvent (Variables|Components|GetBP_ObjectiveCollision) OverlappedComponent OtherActor OtherComp OtherBodyIndex bFromSweep SweepResult)))

(event EventOnDequiped
  ;[1 1 1] Equip/Dequp Logic
  (Development|SetHiddeninGame (Variables|Components|GetHands) true true)
  (Variables|Default|SetZoomedIn true))

(event EventOnEquiped
  ;[1 1 1] Equip/Dequp Logic
  (Development|SetHiddeninGame (Variables|Components|GetHands) false true)
  (CallFunction|HandleZoom))

(event EventBeginPlay
  (Variables|Default|SetProjectile "/Game/_blueprints/Blueprints/Guns/Turret/BP_HookProjectile.BP_HookProjectile_C")
  (Collision|BindEventtoOnComponentBeginOverlap (Variables|Default|GetInteractionZone) (delegate Custom|On%20Component%20Begin%20Overlap)))

(event Input|ActionEvents|InputActionSecondaryAction
  (params (Key :type Key%20Structure))
  ;[1 1 1] Fire Control
  ;;[1 1 1] RMB to zoom toggle
  (:Pressed
    (if (not (or (Variables|Default|GetIsZoomingIn) (Variables|Default|GetIsReloading)))
      (CallFunction|HandleZoom))))

(event Input|AxisEvents|InputAxisMoveRight/Left
  (params (AxisValue :type Float%20%28single-precision%29))
  (bind _returnvalue (Math|Float|Clamp(Float) AxisValue -0.1 0.1))
  ;[1 1 1] Move the Yaw of the turret
  (if (not (Variables|Default|GetIsReloading))
    (Utilities|IsWithinBounds (Variables|Default|GetMinYawVal) (Variables|Default|GetMaxYawVal) (+ _returnvalue (.yaw (Transformation|GetActorRotation)))
      (:true
        (Pawn|Input|AddControllerYawInput _returnvalue)))))

(event Input|AxisEvents|InputAxisLookUp/DownMouse
  (params (AxisValue :type Float%20%28single-precision%29))
  ;[0.05 0.05 0.05] Camera Yaw and Pitch rotation movement
  (if (not (Variables|Default|GetIsReloading))
    (CallFunction|CalculateGunRot AxisValue)))

(event Input|MouseEvents|LeftMouseButton
  (params (Key :type Key%20Structure))
  ;[1 1 1] Fire Control
  (:Pressed
    (CallFunction|FireGun)))

(fn ConstructionScript)

(fn CalculateCamera
  (params (DeltaInput :type Float%20%28double-precision%29))
  (bind _returnvalue (* DeltaInput -1.0))
  (bind _camera (Variables|Default|GetCamera))
  (bind _relativerotation (Variables|/Script/Engine.SceneComponent|GetRelativeRotation _camera))
  (bind _returnvalue_2 (+ _returnvalue (.pitch _relativerotation)))
  (Utilities|IsWithinBounds (Variables|Default|GetMinPitchVal) (Variables|Default|GetMaxPitchVal) _returnvalue_2
    (:true
      (Transformation|SetRelativeRotation (Variables|Default|GetCamera) (Math|Rotator|MakeRotator (.roll _relativerotation) _returnvalue_2 (.yaw _relativerotation)) false false))))

(fn CalculateGunRot
  (params (A :type Float%20%28double-precision%29))
  (bind _gun (Variables|Default|GetGun))
  (bind _relativerotation (Variables|/Script/Engine.SceneComponent|GetRelativeRotation _gun))
  (bind _returnvalue (+ A (.roll _relativerotation)))
  (Utilities|IsWithinBounds (Variables|Default|GetMinPitchVal) (Variables|Default|GetMaxPitchVal) _returnvalue
    (:true
      (Transformation|SetRelativeRotation (Variables|Default|GetGun) (Math|Rotator|MakeRotator _returnvalue (.pitch _relativerotation) (.yaw _relativerotation)) false false))))

(fn AimDownSightLogic
  (params (Alpha :type Float%20%28single-precision%29))
  (bind _aimdownsight (Variables|Components|GetAimDownSight))
  (bind _relativelocation (Variables|/Script/Engine.SceneComponent|GetRelativeLocation _aimdownsight))
  (if (not (Variables|Default|GetZoomedIn))
    (Transformation|SetRelativeLocation (Variables|Default|GetCamera) (Math|Vector|Lerp(Vector) (Variables|/Script/Engine.SceneComponent|GetRelativeLocation (Variables|Default|GetCamera)) (Variables|/Script/Engine.SceneComponent|GetRelativeLocation (Variables|Components|GetAimDownSight)) Alpha) false false)
    (else
      (Transformation|SetRelativeLocation (Variables|Default|GetCamera) (Math|Vector|Lerp(Vector) _relativelocation (+ _relativelocation "0.000000,-140.000000,28.000000") Alpha) false false))))

(fn SetupCameraforAimDown
  (bind _camera (Variables|Default|GetCamera))
  (if (Variables|Default|GetZoomedIn)
    ;[1 1 1] Should remove because redundant but need to go into inherited turretbase to remove old camera and all that, plus camera rotation woes
    (Transformation|AttachComponentToComponent (Variables|Default|GetCamera) (Variables|Default|GetGun) "None" "KeepWorld" "SnapToTarget" "KeepRelative" false)
    (Transformation|SetRelativeRotation _camera "-7.500000,90.000000,0.000000" false false)
    (else
      (Transformation|AttachComponentToComponent (Variables|Default|GetCamera) (Variables|Default|GetGun) "None" "KeepWorld" "SnapToTarget" "KeepRelative" true)
      (Transformation|SetRelativeRotation _camera "-6.500000,90.000000,0.000000" false false))))

(fn ConfigureProjectile
  (params (Object :type Object%20Object%20Reference))
  (bind _asbp_hook_projectile (Utilities|Casting|CastToBP_HookProjectile Object))
  (Variables|Default|Setgrapple_hook _asbp_hook_projectile))

(fn TargetHit
  (params (target :type Vector))
  (Audio|PlaySound2D "/Game/_assets/audio/Prof/CannonSequence/Great_Job.Great_Job" 1.3 1.0 0.0 0 0)
  (Variables|Default|SetisEquippable false)
  (Development|SetHiddeninGame (Variables|Components|GetHands) true false)
  (Default|StartZiplining (Variables|Default|GetZiplineManager) target)
  (CallFunction|Dequip))

(fn TargetMissed
  ;[1 1 1] Lowered volume and increased start time
  (Audio|PlaySound2D "/Game/_assets/audio/Prof/CannonSequence/Aim_For_The_Smokestack.Aim_For_The_Smokestack" 0.04 1.0 0.4 0 0))