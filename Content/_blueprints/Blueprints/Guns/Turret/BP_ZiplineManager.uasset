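; BP_ZiplineManager moves the player along a zipline after leaving a turret.
; StartZiplining stores the target, gets the player character and waits briefly for it to be removed from the turret.
; Two chained timelines then lerp the player's location without sweep, first to a socket on the attached grapple's attach point, then on to the zipline target.
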(event Custom|StartZiplining
  (params (Target :type Vector))
  (Variables|Default|SetTarget Target)
  (Variables|Default|Setplayer (Game|GetPlayerCharacter 0))
  ;[1 1 1] Delay to wait until palyer is removed from turret
  (Utilities|FlowControl|Delay 0.3)
  ;[1 1 1] Lerp from turret to attach point
  (Variables|Default|SetInitialPos (Transformation|GetActorLocation (Variables|Default|Getplayer)))
  (bind _newtrack_0 (Timeline|LerpToAttachedGrapple PlayFromStart)
    (:Update
      (Transformation|SetActorLocation (Variables|Default|Getplayer) (Math|Vector|Lerp(Vector) (Variables|Default|GetInitialPos) (Transformation|GetSocketLocation (Variables|/Game/_blueprints/Blueprints/Guns/Turret/BP_AttachGrapple.BP_AttachGrapple_C|GetAttachPoint (Variables|Default|GetAttachGrapple)) "joint1") _newtrack_0) false false))
    (:Finished
      (Variables|Default|SetInitialPos (Transformation|GetActorLocation (Variables|Default|Getplayer)))
      ;[1 1 1] Lerp to zipline target
      (bind _newtrack_0_2 (Timeline|LerpToEndPoint PlayFromStart)
        (:Update
          (Transformation|SetActorLocation (Variables|Default|Getplayer) (Math|Vector|Lerp(Vector) (Variables|Default|GetInitialPos) (Variables|Default|GetTarget) _newtrack_0_2) false false))))))

(event EventBeginPlay
  ;[1 1 1] Get ref to player just in case turret still is possessed
)

(fn ConstructionScript)