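; Grappling hook projectile fired by BP_GrappleTurret, trailing a cable attached to the turret's gun.
; Overlapping a BP_ValidVolume stops the hook, stores the grapple point and notifies the turret of the hit.
; The cable end then moves to the attach point of the turret's grapple surface, if that is a BP_AttachGrapple.
; A delayed timer handles misses, with TargetMissed destroying the hook and notifying the turret.
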(event OnComponentBeginOverlap(SphereCollision)
  (params (OverlappedComponent :type Primitive%20Component%20Object%20Reference) (OtherActor :type Actor%20Object%20Reference) (OtherComp :type Primitive%20Component%20Object%20Reference) (OtherBodyIndex :type Integer) (bFromSweep :type Boolean) (SweepResult :type Hit%20Result%20Structure%20%28by%20ref%29))
  (Development|PrintString (Utilities|GetDisplayName OtherActor))
  (Utilities|Casting|CastToBP_ValidVolume OtherActor)
  (CallFunction|OnHitTarget)
  (Default|TargetHit (Variables|Default|GetTurret) (Transformation|GetActorLocation))
  (Variables|Default|SetisHit true))

(event Custom|OnHitTarget
  (bind _projectilemovement (Variables|Default|GetProjectileMovement))
  (Components|Movement|StopMovementImmediately _projectilemovement)
  (Variables|/Script/Engine.ProjectileMovementComponent|SetProjectileGravityScale _projectilemovement 0.0)
  (Variables|Default|SetGrapplePoint (Transformation|GetActorLocation))
  (Variables|Default|SetIsGrappled true)
  (bind _asbp_attach_grapple (Utilities|Casting|CastToBP_AttachGrapple (Variables|/Game/_blueprints/Blueprints/Guns/Turret/BP_GrappleTurret.BP_GrappleTurret_C|GetGrappleSurface (Variables|Default|GetTurret))))
  (Class|CableComponent|SetAttachEndtoComponent (Variables|Default|GetCable) (Variables|/Game/_blueprints/Blueprints/Guns/Turret/BP_AttachGrapple.BP_AttachGrapple_C|GetAttachPoint _asbp_attach_grapple) "joint1"))

(event Custom|DestroyIfNotHit
  (if (not (Variables|Default|GetisHit))
    (CallFunction|TargetMissed)))

(event EventBeginPlay
  (bind _asbp_grapple_turret (Utilities|Casting|CastToBP_GrappleTurret (Game|GetInstigator)))
  (Variables|Default|SetTurret _asbp_grapple_turret)
  (Class|CableComponent|SetAttachEndtoComponent (Variables|Default|GetCable) (Variables|/Game/_blueprints/Blueprints/Guns/Turret/Templates/BP_TurretBase.BP_TurretBase_C|GetGun _asbp_grapple_turret) "joint1")
  (Utilities|Time|SetTimerbyEvent (EventDispatchers|CreateEvent :!event Custom|DestroyIfNotHit) 0.1 false 3.0))

(fn ConstructionScript)

(fn TargetMissed
  (Actor|DestroyActor)
  (Default|TargetMissed (Variables|Default|GetTurret)))