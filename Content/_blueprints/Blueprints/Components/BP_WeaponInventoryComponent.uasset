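; Weapon inventory component for BP_FirstPersonCharacter that handles acquiring, swapping, firing and reloading weapons.
; Pickups copy WeaponData table rows into an inventory map and cycle list, which a gate-throttled swap steps through for the primary slot.
; Equipping clears use-weapon bindings and caches the slot's ammo; firing checks it, then sends damage and range to the character's Rifle.
; SMG fires automatically and reloads by montage, while Shotgun uses a looping, fire-interruptible timer.
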(event Custom|TryReloadShotgun
  ;[1 1 1] Reload Logic
  (if (== (Variables|WeaponAmmoData|GetMax%20Ammo) (Variables|WeaponAmmoData|GetAmmo%20Loaded))
    (CallFunction|FinishedReloading)
    (else
      (Animation|Montage|PlayMontage (Variables|/Game/_blueprints/Blueprints/PlayableCharacters/BP_FirstPersonCharacter.BP_FirstPersonCharacter_C|GetFirstPersonMesh (Variables|Components|GetCharRef)) "/Game/_assets/FPHands/Animations/Shotgun/Reload_shotgun_hands_Montage.Reload_shotgun_hands_Montage" 1.1 0.4
        (:then
          (Components|Animation|PlayAnimation (Variables|/Game/_blueprints/Blueprints/PlayableCharacters/BP_FirstPersonCharacter.BP_FirstPersonCharacter_C|GetWeapon (Variables|Components|GetCharRef)) "/Game/_assets/Guns/Shotgun/animation/Reload_shotgun.Reload_shotgun" false))
        (:OnCompleted
          (Math|Integer|IncrementInt (Variables|WeaponAmmoData|GetAmmo%20Loaded)))))))

(event Custom|On%20Drop%20Weapon
  (params (Weapon :type E_Weapon%20Enum :default "NewEnumerator3"))
  ;[1 1 1] Drop Weapon
  (Utilities|Map|Remove (Variables|InventoryData|GetWeaponInventory) Weapon))

(event Custom|WeaponSwap
  (bind _weaponslots (Variables|InventoryData|GetWeaponSlots))
  (bind (_value _returnvalue) (Utilities|Map|Find _weaponslots "NewEnumerator0"))
  ;[1 1 1] Weapon Swap
  ;;[1 1 1] Block Equip Spamming
  (Utilities|FlowControl|Gate false :!label _label
    (:Exit
      (Utilities|FlowControl|Sequence
        (:then_0
          (goto _label Close))
        (:then_1
          (Utilities|FlowControl|Sequence
            (:then_0
              ;;[1 1 1] Increment, modulo, and update enum for primary weapon
              (if _returnvalue
                (Utilities|Map|Add (Variables|InventoryData|GetWeaponSlots) "NewEnumerator0" (Utilities|Array|Get(acopy) (Variables|InventoryData|GetCycleSlots) (Math|Integer|%(Integer) (+ (Utilities|Array|FindItem (Variables|InventoryData|GetCycleSlots) _value) 1) (Utilities|Array|Length (Variables|InventoryData|GetCycleSlots)))))))
            (:then_1
              (CallFunction|WeaponEquip))))
        (:then_2
          (Utilities|FlowControl|Delay 1.0)
          (goto _label Open))))))

(event Custom|WeaponEquip
  ;[1 1 1] Weapon Equipping: Unbind weapons so that only the correct weapon binds it later, also play some swap animation
  (EventDispatchers|UnbindallEventsfromUseWeaponDispatcher)
  (Variables|Default|SetCanFire true)
  (Utilities|SelectedWeaponAmmoInit))

(event Custom|OnAcquireWeapon
  (params (New :type E_Weapon%20Enum :default "NewEnumerator0"))
  (bind _weaponinventory (Variables|InventoryData|GetWeaponInventory))
  (bind _weaponinventory_2 (Variables|InventoryData|GetWeaponInventory))
  (bind (_value _returnvalue) (Utilities|Map|Find _weaponinventory_2 New))
  (bind _weaponstatus (Utilities|Struct|BreakS_WeaponData _value))
  ;[1 1 1] Add Weapon
  (Utilities|FlowControl|Sequence
    (:then_0
      ;;[1 1 1] Find data for this weapon in datatable
      (bind _returnvalue_2 (Utilities|GetDataTableRow "/Game/_blueprints/Blueprints/DataTables/WeaponData.WeaponData" (CallFunction|WeaponEnumtoName New))
        (:then
          (if _returnvalue
            ;;[1 0.706 0.3106] If Weapon is already in inventory, update its stats to original
            (if (Utilities|Struct|BreakS_WeaponStatus _weaponstatus)
              (Utilities|Struct|SetmembersinS_WeaponStatus _weaponstatus (.AmmoHeld (Utilities|Struct|BreakS_WeaponStatus (.WeaponStatus (Utilities|Struct|BreakS_WeaponData _returnvalue_2)))) (.AmmoLoaded (Utilities|Struct|BreakS_WeaponStatus (.WeaponStatus (Utilities|Struct|BreakS_WeaponData _returnvalue_2)))) (.MaxAmmo (Utilities|Struct|BreakS_WeaponStatus (.WeaponStatus (Utilities|Struct|BreakS_WeaponData _returnvalue_2)))))
              (Development|PrintString "Already Have" false)
              (else
                ;;[1 0.06562 0.06562] This doesn't actually do anything
                (Utilities|Struct|SetmembersinS_WeaponStatus (.WeaponStatus (Utilities|Struct|BreakS_WeaponData _returnvalue_2)) true :!label _label)
                (Utilities|Map|Add _weaponinventory New _returnvalue_2)
                (Development|PrintString (Utilities|String|ToString(Integer) (Utilities|Map|Length _weaponinventory)) false)
                (Utilities|Map|Add (Variables|InventoryData|GetWeaponSlots) "NewEnumerator0" New)
                (Utilities|Array|AddUnique (Variables|InventoryData|GetCycleSlots) New)))
            (else
              (goto _label))))
        (:RowNotFound
          (Development|PrintString "Row Not Found" false))))
    (:then_1
      (CallFunction|WeaponEquip))))

(event Custom|EquipCheckUnarmed
  (params (New :type E_Weapon%20Enum :default "NewEnumerator3"))
  ;[1 1 1] Unarmed Strike Setup
  (if (Utilities|Enum|Equal(Enum) New "NewEnumerator3")
    (EventDispatchers|BindEventtoUseWeaponDispatcher (delegate Custom|UnarmedStrike))))

(event Custom|UnarmedStrike
  (params (Damage :type Integer) (Range :type Float%20%28double-precision%29))
  ;[1 1 1] Unarmed Strike Setup
  (Development|PrintString (Utilities|String|Append "Pow:  " (Utilities|String|ToString(Integer) Damage)) false))

(event EventBeginPlay
  (EventDispatchers|BindEventtoEquipWeaponDispatcher (EventDispatchers|CreateEvent :!event Custom|EquipCheckUnarmed)) ; You Start with unarmed ability unlocked
  (bind _asbp_first_person_character (Utilities|Casting|CastToBP_FirstPersonCharacter (Components|GetOwner)))
  (Variables|Components|SetCharRef _asbp_first_person_character))

(event Input|ActionEvents|InputActionPrimaryAction
  (params (Key :type Key%20Structure :default "None"))
  (bind _weaponslots (Variables|InventoryData|GetWeaponSlots))
  (bind (_value _returnvalue) (Utilities|Map|Find _weaponslots "NewEnumerator0"))
  (bind _returnvalue_2 (Utilities|Enum|Equal(Enum) _value "NewEnumerator4"))
  ;[1 1 1] Shooting
  (:Pressed
    (if _returnvalue
      (Utilities|FlowControl|Sequence
        (:then_0
          (if (and (Variables|Default|GetIsReloading) (Utilities|Enum|Equal(Enum) _value "NewEnumerator1"))
            (CallFunction|FinishedReloading)))
        (:then_1
          (if _returnvalue_2
            (bind _success (CallFunction|AutoTryFire))
            (if (not _success)
              (Audio|PlaySound2D "/Game/_assets/audio/Guns/DryFire/R_DryFire.R_DryFire" 1.0 1.0 0.0 0 0 :!label _label))
            (else
              (bind _success_2 (CallFunction|TryFire))
              (if (not _success_2)
                (goto _label))))))))
  (:Released
    (if _returnvalue_2
      (Variables|Default|SetIsAutoFiring false)
      (Variables|Default|SetCanFire true))))

(event Input|ActionEvents|InputActionReload
  (params (Key :type Key%20Structure :default "None"))
  ;[1 1 1] Reload Logic
  (:Pressed
    (if (not (or (Variables|Default|GetIsReloading) (Variables|Default|GetIsAutoFiring)))
      (Variables|Default|SetIsReloading true)
      (Variables|Default|SetCanFire false)
      (switch Utilities|FlowControl|Switch|SwitchonE_Weapon (.Value (Utilities|Map|Find (Variables|InventoryData|GetWeaponSlots) "NewEnumerator0"))
        (:NewEnumerator3
          (Variables|Default|SetIsReloading false :!label _label)
          (Variables|Default|SetCanFire true))
        (:NewEnumerator1
          (bind _returnvalue (Utilities|Time|SetTimerbyEvent (EventDispatchers|CreateEvent :!event Custom|TryReloadShotgun) 0.8 true))
          (Variables|Default|SetReloadTimer _returnvalue))
        (:NewEnumerator4
          (if (== (Variables|WeaponAmmoData|GetMax%20Ammo) (Variables|WeaponAmmoData|GetAmmo%20Loaded))
            (goto _label)
            (else
              (Animation|Montage|PlayMontage (Variables|/Game/_blueprints/Blueprints/PlayableCharacters/BP_FirstPersonCharacter.BP_FirstPersonCharacter_C|GetFirstPersonMesh (Variables|Components|GetCharRef)) "/Game/_assets/FPHands/Animations/Sten/AM_StenReload.AM_StenReload"
                (:then
                  (Components|Animation|PlayAnimation (Variables|/Game/_blueprints/Blueprints/PlayableCharacters/BP_FirstPersonCharacter.BP_FirstPersonCharacter_C|GetWeapon (Variables|Components|GetCharRef)) "/Game/_assets/Guns/Sterling/Animations/Reload.Reload" false))
                (:OnCompleted
                  (Variables|WeaponAmmoData|SetAmmo%20Loaded (Variables|WeaponAmmoData|GetMax%20Ammo))
                  (Variables|Default|SetIsReloading false :!label _label_2)
                  (Variables|Default|SetCanFire true))
                (:OnInterrupted
                  (goto _label_2))))))))))

(event Input|KeyboardEvents|C
  (params (Key :type Key%20Structure :default "None"))
  ;[1 1 1] Weapon Swap
)

(fn CheckGunAmmo
  (bind _ammo_loaded (Variables|WeaponAmmoData|GetAmmo%20Loaded))
  (bind _returnvalue (> _ammo_loaded 0))
  (if _returnvalue
    (return true)
    (else
      (return (or _returnvalue (< (Variables|WeaponAmmoData|GetMax%20Ammo) 0))))))

(fn GetWeaponData
  (params (Key :type E_Slots%20Enum%20%28by%20ref%29 :default "NewEnumerator0"))
  (return (.Value (Utilities|Map|Find (Variables|InventoryData|GetWeaponInventory) (.Value (Utilities|Map|Find (Variables|InventoryData|GetWeaponSlots) Key))))))

(fn TryFire
  (bind (_damage _range) (CallFunction|GetWeaponRangeDamage "NewEnumerator0"))
  (if (Variables|Default|GetCanFire)
    (if (CallFunction|CheckGunAmmo)
      (Default|SetRangeDamage (Variables|/Game/_blueprints/Blueprints/PlayableCharacters/BP_FirstPersonCharacter.BP_FirstPersonCharacter_C|Getrifle (Variables|Components|GetCharRef)) _damage _range)
      (Variables|Default|SetCanFire false)
      (return true)
      (else
        _)))
  (return false))

(fn GetWeaponRangeDamage
  (params (WeaponSlot :type E_Slots%20Enum :default "NewEnumerator0"))
  (bind _value (CallFunction|GetWeaponData WeaponSlot))
  (bind (_basedamage _tracerange) (Utilities|Struct|BreakS_WeaponData _value))
  (return _basedamage _tracerange))

(fn SetWeaponData
  (params (Key :type E_Slots%20Enum%20%28by%20ref%29 :default "NewEnumerator0"))
  (return (.Value (Utilities|Map|Find (Variables|InventoryData|GetWeaponInventory) (.Value (Utilities|Map|Find (Variables|InventoryData|GetWeaponSlots) Key))))))

(fn UpdateAmmoCount)

(fn AutoTryFire
  (bind (_damage _range) (CallFunction|GetWeaponRangeDamage "NewEnumerator0"))
  (if (Variables|Default|GetCanFire)
    (if (CallFunction|CheckGunAmmo)
      (Variables|Default|SetIsAutoFiring true)
      (Default|SetRangeDamage (Variables|/Game/_blueprints/Blueprints/PlayableCharacters/BP_FirstPersonCharacter.BP_FirstPersonCharacter_C|Getrifle (Variables|Components|GetCharRef)) _damage _range)
      (return true)
      (else
        _)))
  (return false))

(fn DecrementAmmo
  (Variables|WeaponAmmoData|SetAmmo%20Loaded (- (Variables|WeaponAmmoData|GetAmmo%20Loaded) 1)))

(fn FinishedReloading
  (Utilities|Time|ClearandInvalidateTimerbyHandle (Variables|Default|GetReloadTimer))
  (Variables|Default|SetIsReloading false)
  (Variables|Default|SetCanFire true))