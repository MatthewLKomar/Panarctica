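; BP_PawnHealthComponent is a pawn component that tracks health, applies damage and regenerates health over time.
; ApplyDamage lowers health unless IsGod is set, fires OnDamage, starts the regen delay and calls Death at zero or below.
; A retriggerable delay restarts on each hit, then resumes a looping timer and fires OnRecovery.
; The timer, created paused at BeginPlay, adds rate-scaled health each tick and pauses itself at MaxHealth.
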(event Custom|ApplyDamage
  (params (Damage :type Float%20%28double-precision%29) (FromDamage :type Vector))
  ;[1 1 1] Apply Damage to self
  (if (not (Variables|Default|GetisGod))
    (bind _output_get (Variables|Default|SetHealth (- (Variables|Default|GetHealth) Damage)))
    (Default|CallOnDamage Damage)
    (CallFunction|DelayRegen)
    (if (<= _output_get 0.0)
      (Default|CallDeath))))

(event Custom|DelayRegen
  ;[1 1 1] Pause regen
  (Utilities|FlowControl|RetriggerableDelay (Variables|Default|GetRegenDelay))
  (CallFunction|RegenHealth)
  (Utilities|Time|UnpauseTimerbyHandle (Variables|Default|GetRegenTimer))
  (Default|CallOnRecovery))

(event Custom|RegenHealth
  (bind _maxhealth (Variables|Default|GetMaxHealth))
  ;[1 1 1] Regen Health
  (if (>= (+ (Variables|Default|Gethealth) (* (Variables|Default|GetRegenPeriod) (Variables|Default|GetRegenRate))) _maxhealth)
    (Variables|Default|Sethealth _maxhealth)
    (Utilities|Time|PauseTimerbyHandle (Variables|Default|GetRegenTimer))
    (else
      (Variables|Default|Sethealth (+ (Variables|Default|Gethealth) (* (Variables|Default|GetRegenPeriod) (Variables|Default|GetRegenRate)))))))

(event EventBeginPlay
  (Variables|Default|SetHealth (Variables|Default|GetMaxHealth))
  (if (> (Variables|Default|GetRegenRate) 0.0)
    (bind _returnvalue (Utilities|Time|SetTimerbyEvent (delegate Custom|RegenHealth) (Variables|Default|GetRegenPeriod) true))
    (bind _output_get (Variables|Default|SetRegenTimer _returnvalue))
    (Utilities|Time|PauseTimerbyHandle _output_get)))