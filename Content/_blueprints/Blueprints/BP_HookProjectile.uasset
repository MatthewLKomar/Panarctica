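; Grappling hook projectile that trails a cable back to the gun that uses it.
; On BeginPlay it adds a cable component with its end attached to the Muzzle socket on the Gun's skeletal mesh.
; When OnHitTarget fires, it halts projectile movement, removes gravity, stores its location as the grapple point and flags itself as grappled.
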(event Custom|OnHitTarget
  (bind _projectilemovement (Variables|Default|GetProjectileMovement))
  (Components|Movement|StopMovementImmediately _projectilemovement)
  (Variables|/Script/Engine.ProjectileMovementComponent|SetProjectileGravityScale _projectilemovement 0.0)
  (Variables|Default|SetGrapplePoint (Transformation|GetActorLocation))
  (Variables|Default|SetIsGrappled true))

(event EventBeginPlay
  (bind _returnvalue (AddComponent|AddCableComponent false))
  (bind _output_get (Variables|Default|SetGrappleCable _returnvalue))
  (Class|CableComponent|SetAttachEndto _output_get (Variables|Default|GetGun) "SkeletalMesh" "Muzzle"))

(event Collision|EventActorBeginOverlap
  (params (OtherActor :type Actor%20Object%20Reference)))

(event EventTick
  (params (DeltaSeconds :type Float%20%28single-precision%29)))

(fn ConstructionScript)